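; BP_DMSPlayerController is a player controller with a helper for moving the mouse cursor with a gamepad thumbstick.
; ControlMouseViaThumbstick adds scaled input axis values to the current mouse position, rounds the result and sets it as the new cursor location.
; The helper's call is disconnected from any event, and the IA_Look, BeginPlay and Tick events are empty, so the controller currently runs no logic.
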(event Input|EnhancedActionEvents|EnhancedInputActionIA_Look
  (params (ActionValue :type Vector%202D%20Structure) (ElapsedSeconds :type Float%20%28double-precision%29) (TriggeredSeconds :type Float%20%28double-precision%29) (InputAction :type Input%20Action%20Object%20Reference :default "/Game/Blueprints/Input/InputActions/IA_Look.IA_Look")))

(event EventBeginPlay)

(event EventTick
  (params (DeltaSeconds :type Float%20%28single-precision%29)))

(fn ConstructionScript)

(fn ControlMouseViaThumbstick
  (bind _returnvalue (Game|GetPlayerController 0))
  (bind (_locationx _locationy) (Game|Player|GetMousePosition _returnvalue))
  (Class|PlayerController|SetMouseLocation (Game|GetPlayerController 0) (Math|Float|Round (+ (* (Class|Actor|GetInputAxisKeyValue) 12.0) _locationx)) (Math|Float|Round (+ (* (Class|Actor|GetInputAxisKeyValue) 12.0) _locationy))))